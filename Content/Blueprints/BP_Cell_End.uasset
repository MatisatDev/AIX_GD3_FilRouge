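; End cell Blueprint that announces the game result when its Action runs.
; It extends the parent cell's Action, then compares the Score of the first two players in the game instance's PlayerList, ignoring PlayerID.
; A two-step sequence prints which player wins, and both false branches share one equality check, so a tie prints "égalité" twice.
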(fn `Action`
  (params (PlayerID :type Integer))
  (bind (_playerid _score) (break `/Game/Blueprints/S_PlayerData` (`|GetArrayItem` (`/Game/Blueprints/BP_GameInstance.PlayerList` (`self.As BP Game Instance`)) 1)))
  (bind (_playerid_2 _score_2) (break `/Game/Blueprints/S_PlayerData` (`|GetArrayItem` (`/Game/Blueprints/BP_GameInstance.PlayerList` (`self.As BP Game Instance`)))))
  (`parent.Action` PlayerID)
  (`|ExecutionSequence`
    (:`then_0`
      (if (> _score_2 _score)
        (`KismetSystemLibrary.PrintString` "Player 1 Win !")
        (else
          (if (== _score _score_2) :!label _label
            (`KismetSystemLibrary.PrintString` "égalité")))))
    (:`then_1`
      (if (< _score_2 _score)
        (`KismetSystemLibrary.PrintString` "Player 2 win !")
        (else
          (goto _label))))))

(fn `UserConstructionScript`
  (`parent.UserConstructionScript`))